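; Sunshine is a proximity hazard actor that ends the game when the player gets too close and shows itself when hit by a probe scan.
; Tick checks distance to the player pawn, pausing the game and adding the LostMenu widget when within range.
; A pair of DoOnce nodes limits this to once per approach, re-arming after the player leaves range.
; ProbeScanHit unhides the actor, then a retriggerable delay hides it again.
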(event `self.ReceiveTick`
  (params (DeltaSeconds :type "Float (single-precision)"))
  (if (< (`self.GetDistanceTo` (`GameplayStatics.GetPlayerPawn` 0)) 165.0)
    (`/Engine/EditorBlueprintResources/StandardMacros.DoOnce` false :!label _label
      (:`Completed`
        (`|ExecutionSequence`
          (:`then_0`
            (goto _label_2 :!via `Reset`))
          (:`then_1`
            (bind _returnvalue (`|CreateWidget` "/Game/UI/Game_Over_Widget/Start_Widget/LostMenu.LostMenu_C"))
            (`GameplayStatics.SetGamePaused` true)
            (`UserWidget.AddToViewport` _returnvalue 0)))))
    (else
      (`/Engine/EditorBlueprintResources/StandardMacros.DoOnce` false :!label _label_2
        (:`Completed`
          (goto _label :!via `Reset`))))))

(event `/Game/Blueprints/Triggers.ProbeScanHit`
  (params (ProbePosition :type "Vector Structure"))
  (`self.SetActorHiddenInGame` false)
  (`KismetSystemLibrary.RetriggerableDelay` 3.0)
  (`self.SetActorHiddenInGame` true))

(fn `UserConstructionScript`)