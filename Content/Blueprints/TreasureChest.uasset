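; Treasure chest actor that serves as the level's win goal and appears when the player is near or a probe scan reaches it.
; A probe scan reveals it for three retriggerable seconds if a line trace to the probe finds no WorldStatic blocker.
; Tick tracks player distance, using paired DoOnce gates to toggle visibility on range changes.
; At closer range, it pauses the game and shows the win menu once.
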(event `/Game/Blueprints/Triggers.ProbeScanHit`
  (params (ProbePosition :type "Vector Structure"))
  (bind (_outhit _returnvalue) (`KismetSystemLibrary.LineTraceSingleForObjects` (`self.K2_GetActorLocation`) ProbePosition (`|MakeArray` "ObjectTypeQuery1" :!type "EObjectTypeQuery Enum")))
  (if (not _returnvalue)
    (`self.SetActorHiddenInGame` false)
    (`KismetSystemLibrary.RetriggerableDelay` 3.0)
    (`self.SetActorHiddenInGame` true)))

(event `self.ReceiveTick`
  (params (DeltaSeconds :type "Float (single-precision)"))
  (bind _returnvalue (`self.GetDistanceTo` (`GameplayStatics.GetPlayerPawn` 0)))
  (set `self.TreasureDistance` _returnvalue)
  (if (< _returnvalue 750.0)
    (`|ExecutionSequence`
      (:`then_0`
        (`/Engine/EditorBlueprintResources/StandardMacros.DoOnce` false :!label _label
          (:`Completed`
            (`self.SetActorHiddenInGame` false)
            (goto _label_2 :!via `Reset`))))
      (:`then_1`
        (if (< _returnvalue 360.0)
          (`/Engine/EditorBlueprintResources/StandardMacros.DoOnce` false
            (:`Completed`
              (bind _returnvalue_2 (`|CreateWidget` "/Game/UI/Game_Over_Widget/Start_Widget/WinMenu2.WinMenu2_C"))
              (`GameplayStatics.SetGamePaused` true)
              (`UserWidget.AddToViewport` _returnvalue_2 0))))))
    (else
      (`/Engine/EditorBlueprintResources/StandardMacros.DoOnce` false :!label _label_2
        (:`Completed`
          (`self.SetActorHiddenInGame` true)
          (goto _label :!via `Reset`))))))

(fn `UserConstructionScript`)