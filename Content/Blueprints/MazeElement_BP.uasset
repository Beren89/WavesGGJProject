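; MazeElement is a maze piece Blueprint that displays a configurable Paper2D sprite, applied in the construction script.
; On ProbeScanHit it traces WorldStatic objects from itself to the probe position, with persistent debug drawing.
; If the hit actor is not hidden, it unhides itself, then hides again after a retriggerable three-second delay.
; The trace's boolean result is unused.
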(event `/Game/Blueprints/Triggers.ProbeScanHit`
  (params (ProbePosition :type "Vector Structure"))
  (bind (_outhit _returnvalue) (`KismetSystemLibrary.LineTraceSingleForObjects` :`Start` (`self.K2_GetActorLocation`) :`End` ProbePosition :`ObjectTypes` (`|MakeArray` "ObjectTypeQuery1" :!type "EObjectTypeQuery Enum") :`DrawDebugType` "Persistent"))
  (if (not (`Actor.bHidden` (`.HitActor` (`GameplayStatics.BreakHitResult` _outhit))))
    (`self.SetActorHiddenInGame` false)
    (`KismetSystemLibrary.RetriggerableDelay` 3.0)
    (`self.SetActorHiddenInGame` true)))

(fn `UserConstructionScript`
  (`PaperSpriteComponent.SetSprite` (`self.PaperSprite`) (`self.Sprite`)))