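; Probe actor that emits an expanding scan pulse and notifies the actors it reaches.
; Each Tick grows the capsule radius by a fixed, frame-rate-dependent step and scales the Paper sprite to match.
; Each overlapped actor receives a ProbeScanHitMessage carrying the probe's location.
; The probe destroys itself once its radius nears MaximumRadius.
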(event `self.ReceiveActorBeginOverlap`
  (params (OtherActor :type "Actor Object Reference"))
  (message `/Game/Blueprints/Triggers.ProbeScanHit` OtherActor (`self.K2_GetActorLocation`)))

(event `self.ReceiveTick`
  (params (DeltaSeconds :type "Float (single-precision)"))
  (bind _returnvalue (+ (`self.CurrentRadius`) 5.0))
  (bind _returnvalue_2 (/ _returnvalue 400.0))
  (`CapsuleComponent.SetCapsuleRadius` (`self.Capsule`) _returnvalue true)
  (`SceneComponent.SetWorldScale3D` (`self.PaperSprite`) (`KismetMathLibrary.MakeVector` _returnvalue_2 0.0 _returnvalue_2))
  (bind _output_get (set `self.CurrentRadius` _returnvalue))
  (if (`KismetMathLibrary.NearlyEqual_FloatFloat` _output_get (`self.MaximumRadius`) 5.0)
    (`self.K2_DestroyActor`)))

(fn `UserConstructionScript`)